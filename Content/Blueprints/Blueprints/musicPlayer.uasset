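; Music player Blueprint that keeps background music running from a pool of six Mario Party 9 and Legend of Zelda tracks.
; BeginPlay lowers the volume of the Master audio component.
; Tick polls Master and, whenever it is not playing, assigns a randomly chosen track and plays it from the start, so the same track can repeat back to back.
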(event EventTick
  (params (DeltaSeconds :type Float%20%28single-precision%29))
  (bind _master (Variables|Default|Getmaster))
  (if (not (Audio|Components|Audio|IsPlaying (Variables|Default|Getmaster)))
    (switch int (Math|Random|RandomInteger 6)
      (:0
        (Audio|Components|Audio|SetSound _master "/Game/Sound/Music/Dont_Panic◆Mario_Party_9_Music.Dont_Panic◆Mario_Party_9_Music"))
      (:1
        (Audio|Components|Audio|SetSound _master "/Game/Sound/Music/How_Strange__-_Mario_Party_9.How_Strange__-_Mario_Party_9"))
      (:2
        (Audio|Components|Audio|SetSound _master "/Game/Sound/Music/Hurry_Up_◆Mario_Party_9_Music.Hurry_Up_◆Mario_Party_9_Music"))
      (:3
        (Audio|Components|Audio|SetSound _master "/Game/Sound/Music/Mario_Party_9_-_Stage_Event_Weve_Got_Trouble_.Mario_Party_9_-_Stage_Event_Weve_Got_Trouble_"))
      (:4
        (Audio|Components|Audio|SetSound _master "/Game/Sound/Music/Mini_Game_-_The_Legend_of_Zelda_Ocarina_of_Time.Mini_Game_-_The_Legend_of_Zelda_Ocarina_of_Time"))
      (:5
        (Audio|Components|Audio|SetSound _master "/Game/Sound/Music/Minigame_-_The_Legend_of_Zelda__A_Link_Between_Worlds.Minigame_-_The_Legend_of_Zelda__A_Link_Between_Worlds")))
    (Audio|Components|Audio|Play (Variables|Default|Getmaster) 0.0)))

(event EventBeginPlay
  (Audio|Components|Audio|SetVolumeMultiplier (Variables|Default|Getmaster) 0.15 :!class /Script/Engine.AudioComponent))

(fn ConstructionScript)