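; An actor that shows a world-space fuel progress bar widget facing the player camera.
; On BeginPlay it casts the Bar component's user widget to fuelProgressWidget and stores it as ProgressWidget.
; Each tick, a Billboard function rotates the Bar toward the player camera using a look-at rotation, once the camera manager is valid.
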(event EventTick
  (params (DeltaSeconds :type Float%20%28single-precision%29))
  (CallFunction|Billboard))

(event EventBeginPlay
  (bind _asfuel_progress_widget (Utilities|Casting|CastTofuelProgressWidget (UserInterface|GetUserWidgetObject (Variables|Default|Getbar))))
  (Variables|Default|SetprogressWidget _asfuel_progress_widget))

(fn ConstructionScript)

(fn Billboard
  (bind _returnvalue (Game|GetPlayerCameraManager 0))
  (Utilities|IsValid _returnvalue
    (:Is%20Valid
      (Transformation|SetWorldRotation (Variables|Default|Getbar) (Math|Rotator|FindLookatRotation (Transformation|GetWorldLocation (Variables|Default|Getbar)) (Camera|GetCameraLocation _returnvalue)) false false))))