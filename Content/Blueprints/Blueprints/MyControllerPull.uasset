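; Blueprint that reacts to controller connection changes, pausing the game while a controller is disconnected.
; On disconnect it creates a ReconnectController widget, stores and displays it, passes it the controller ID, and pauses the game.
; On connect it removes the stored widget and unpauses, and every change prints the ID and connection state for debugging.
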(event EventBeginPlay)

(event Collision|EventActorBeginOverlap
  (params (OtherActor :type Actor%20Object%20Reference)))

(event EventTick
  (params (DeltaSeconds :type Float%20%28single-precision%29)))

(event EventOnControllerConnectionChange
  (params (Connected :type Boolean) (UserID :type Integer) (ControllerID :type Integer))
  (Development|PrintString (Class|KismetStringLibrary|BuildStringBool (Utilities|String|ToString(Integer) ControllerID) "" Connected))
  (if Connected
    (Widget|RemovefromParent (stale _output_get))
    (Game|SetGamePaused false)
    (else
      (bind _returnvalue (UserInterface|CreateWidget "/Game/Blueprints/Blueprints/ReconnectController.ReconnectController_C"))
      (bind _output_get (Variables|Default|SetReference%20to%20Widget%20Blueprint _returnvalue))
      (UserInterface|Viewport|AddtoViewport _output_get 0)
      (bind _asreconnect_controller (Utilities|Casting|CastToReconnectController _returnvalue))
      (Variables|/Game/Blueprints/Blueprints/ReconnectController.ReconnectController_C|SetControllerNum _asreconnect_controller ControllerID)
      (Game|SetGamePaused true))))

(fn ConstructionScript)