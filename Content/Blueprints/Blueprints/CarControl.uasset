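; Customer car for a repair shop game that drives in with randomly missing tires and needing paint, then leaves once fixed.
; On BeginPlay it hides up to three tires and timeline-lerps between tagged Point actors to the shop floor.
; Overlapping PickupTire and ColorPaint actors restore parts and consume the pickup.
; Tick checks completion, then drives the car out and destroys it; characters hit while it moves go to time out.
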(event OnComponentBeginOverlap(FRCollider)
  (params (OverlappedComponent :type Primitive%20Component%20Object%20Reference) (OtherActor :type Actor%20Object%20Reference) (OtherComp :type Primitive%20Component%20Object%20Reference) (OtherBodyIndex :type Integer) (bFromSweep :type Boolean) (SweepResult :type Hit%20Result%20Structure%20%28by%20ref%29))
  ;[1 1 1] Placing the Tires down, starting thier destroy function
  (if (Variables|Default|GetFRMissing)
    (if (Utilities|ClassIsChildOf (Utilities|GetClass OtherActor) "/Game/Blueprints/Blueprints/pickupTire.pickupTire_C")
      (CallFunction|EnableFrontRight)
      (bind _aspickup_tire (Utilities|Casting|CastTopickupTire OtherActor))
      (Default|DestroyTire _aspickup_tire))))

(event OnComponentBeginOverlap(FLCollider)
  (params (OverlappedComponent :type Primitive%20Component%20Object%20Reference) (OtherActor :type Actor%20Object%20Reference) (OtherComp :type Primitive%20Component%20Object%20Reference) (OtherBodyIndex :type Integer) (bFromSweep :type Boolean) (SweepResult :type Hit%20Result%20Structure%20%28by%20ref%29))
  ;[1 1 1] Placing the Tires down, starting thier destroy function
  (if (Variables|Default|GetFLMissing)
    (if (Utilities|ClassIsChildOf (Utilities|GetClass OtherActor) "/Game/Blueprints/Blueprints/pickupTire.pickupTire_C")
      (CallFunction|EnableFrontLeft)
      (bind _aspickup_tire (Utilities|Casting|CastTopickupTire OtherActor))
      (Default|DestroyTire _aspickup_tire))))

(event OnComponentBeginOverlap(mainBody)
  (params (OverlappedComponent :type Primitive%20Component%20Object%20Reference) (OtherActor :type Actor%20Object%20Reference) (OtherComp :type Primitive%20Component%20Object%20Reference) (OtherBodyIndex :type Integer) (bFromSweep :type Boolean) (SweepResult :type Hit%20Result%20Structure%20%28by%20ref%29))
  (if (Variables|Default|GetcolorMissing)
    (if (Utilities|ClassIsChildOf (Utilities|GetClass OtherActor) "/Game/Blueprints/Blueprints/colorPaint.colorPaint_C")
      (bind _ascolor_paint (Utilities|Casting|CastTocolorPaint OtherActor))
      (bind _paintmat (Default|ReturnMat _ascolor_paint))
      (CallFunction|SetMat _paintmat)
      (Default|DestroyPaint _ascolor_paint))))

(event OnComponentBeginOverlap(BRCollider)
  (params (OverlappedComponent :type Primitive%20Component%20Object%20Reference) (OtherActor :type Actor%20Object%20Reference) (OtherComp :type Primitive%20Component%20Object%20Reference) (OtherBodyIndex :type Integer) (bFromSweep :type Boolean) (SweepResult :type Hit%20Result%20Structure%20%28by%20ref%29))
  ;[1 1 1] Placing the Tires down, starting thier destroy function
  (if (Variables|Default|GetBRMissing)
    (if (Utilities|ClassIsChildOf (Utilities|GetClass OtherActor) "/Game/Blueprints/Blueprints/pickupTire.pickupTire_C")
      (CallFunction|EnableBackRight)
      (bind _aspickup_tire (Utilities|Casting|CastTopickupTire OtherActor))
      (Default|DestroyTire _aspickup_tire))))

(event OnComponentBeginOverlap(BLCollider)
  (params (OverlappedComponent :type Primitive%20Component%20Object%20Reference) (OtherActor :type Actor%20Object%20Reference) (OtherComp :type Primitive%20Component%20Object%20Reference) (OtherBodyIndex :type Integer) (bFromSweep :type Boolean) (SweepResult :type Hit%20Result%20Structure%20%28by%20ref%29))
  ;[1 1 1] Placing the Tires down, starting thier destroy function
  (if (Variables|Default|GetBLMissing)
    (if (Utilities|ClassIsChildOf (Utilities|GetClass OtherActor) "/Game/Blueprints/Blueprints/pickupTire.pickupTire_C")
      (CallFunction|EnableBackLeft)
      (bind _aspickup_tire (Utilities|Casting|CastTopickupTire OtherActor))
      (Default|DestroyTire _aspickup_tire))))

(event Collision|EventHit
  (params (MyComp :type Primitive%20Component%20Object%20Reference) (Other :type Actor%20Object%20Reference) (OtherComp :type Primitive%20Component%20Object%20Reference) (bSelfMoved :type Boolean) (HitLocation :type Vector :default "0, 0, 0") (HitNormal :type Vector :default "0, 0, 0") (NormalImpulse :type Vector :default "0, 0, 0") (Hit :type Hit%20Result%20Structure%20%28by%20ref%29))
  ;[1 1 1] Timing out Hit Players
  (if (Variables|Default|GetisMoving)
    (if (Utilities|ClassIsChildOf (Utilities|GetClass Other) "/Game/Blueprints/Blueprints/ThirdPersonCharacter.ThirdPersonCharacter_C")
      (bind _asthird_person_character (Utilities|Casting|CastToThirdPersonCharacter Other))
      (Default|GotoTimeOut _asthird_person_character))))

(event EventBeginPlay
  (Utilities|FlowControl|Sequence
    (:then_0
      ;[1 1 1] Set Tires
      (Variables|Default|SetTires (Utilities|Array|MakeArray (Variables|Default|GetFrontRight) (Variables|Default|GetFrontLeft) (Variables|Default|GetBackRight) (Variables|Default|GetBackLeft)))
      (CallFunction|RandomizeTires))
    (:then_1
      ;[1 1 1] Grabbing Car Movement Points
      (bind _outactors (Actor|GetAllActorsOfClass "/Game/Blueprints/Blueprints/Point.Point_C"))
      (for _array_element _outactors
        (Utilities|FlowControl|Sequence
          (:then_0
            (if (Actor|ActorHasTag _array_element "End")
              (Variables|Default|SetEndPoint _array_element)))
          (:then_1
            (if (Actor|ActorHasTag _array_element "Floor")
              (Variables|Default|SetFloorPoint _array_element)))
          (:then_2
            (if (Actor|ActorHasTag _array_element "Start")
              (Variables|Default|SetStartPoint _array_element))))))
    (:then_2
      ;[1 1 1] Lerp from start to shop Floor
      (bind _alpha (Timeline|DriveIN Play)
        (:Update
          (Transformation|SetActorLocation (Math|Vector|Lerp(Vector) (Transformation|GetActorLocation (Variables|Default|GetStartPoint)) (Transformation|GetActorLocation (Variables|Default|GetFloorPoint)) _alpha) false false))
        (:Finished
          (Variables|Default|SetisMoving false))))
    (:then_3
      (Rendering|Material|SetMaterial (Variables|Default|GetmainBody) 0 "/Game/StarterContent/Materials/M_Brick_Clay_New.M_Brick_Clay_New"))))

(event EventTick
  (params (DeltaSeconds :type Float%20%28single-precision%29))
  ;[1 1 1] Checking if car is ready to go
  (CallFunction|CheckDone)
  (if (Variables|Default|GetisLeaving)
    (Variables|Default|SetisMoving true)
    (bind _alpha (Timeline|DriveOut Play)
      (:Update
        (Transformation|SetActorLocation (Math|Vector|Lerp(Vector) (Transformation|GetActorLocation (Variables|Default|GetFloorPoint)) (Transformation|GetActorLocation (Variables|Default|GetEndPoint)) _alpha) false false))
      (:Finished
        (Actor|DestroyActor)))))

(fn ConstructionScript)

(fn RandomizeTires
  (bind _array_element (Utilities|Array|ForEachLoopwithBreak (Variables|Default|GetTires) :!label _label)
    (:LoopBody
      (if (>= (Variables|Default|GetnumDisabledTires) 3) ; If Num of tires off not exceeded
        (goto _label Break)
        (elif (not (Math|Random|RandomBool)) ; If the Random bool is false
          (Rendering|SetVisibility _array_element false true)
          (Variables|Default|SetnumDisabledTires (+ (Variables|Default|GetnumDisabledTires) 1))
          (Utilities|FlowControl|Sequence
            (:then_0
              (if (Utilities|Enum|Equal(Enum) (Utilities|GetObjectName _array_element) "FrontRight")
                (Variables|Default|SetFRMissing true)))
            (:then_1
              (if (Utilities|Enum|Equal(Enum) (Utilities|GetObjectName _array_element) "FrontLeft")
                (Variables|Default|SetFLMissing true)))
            (:then_2
              (if (Utilities|Enum|Equal(Enum) (Utilities|GetObjectName _array_element) "BackRight")
                (Variables|Default|SetBRMissing true)))
            (:then_3
              (if (Utilities|Enum|Equal(Enum) (Utilities|GetObjectName _array_element) "BackLeft")
                (Variables|Default|SetBLMissing true)))))))))

(fn EnableFrontRight
  (Rendering|SetVisibility (Variables|Default|GetFrontRight) true true)
  (Variables|Default|SetFRMissing false))

(fn EnableFrontLeft
  (Rendering|SetVisibility (Variables|Default|GetFrontLeft) true true)
  (Variables|Default|SetFLMissing false))

(fn EnableBackRight
  (Rendering|SetVisibility (Variables|Default|GetBackRight) true true)
  (Variables|Default|SetBRMissing false))

(fn EnableBackLeft
  (Rendering|SetVisibility (Variables|Default|GetBackLeft) true true)
  (Variables|Default|SetBLMissing false))

(fn CheckDone
  (if (Math|Boolean|ANDBoolean (not (Variables|Default|GetFRMissing)) (not (Variables|Default|GetFLMissing)) (not (Variables|Default|GetBRMissing)) (not (Variables|Default|GetBLMissing)) (not (Variables|Default|GetcolorMissing)))
    (Variables|Default|SetisLeaving true)))

(fn SetMat
  (params (newMat :type Material%20Interface%20Object%20Reference))
  (Rendering|Material|SetMaterial (Variables|Default|GetmainBody) 0 newMat)
  (Variables|Default|SetcolorMissing false))