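; Wrench target actor that the player hits a required number of times, tracking the hits left.
; Overlap registers it as the ThirdPersonCharacter's WrenchTarget, and tryHit decrements the count while that player is near.
; Each hit updates a remaining/total widget, which turns to face the camera every tick, and plays a sound at world origin.
; NeedsHits clears only on an update after the count has already reached zero.
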(event Custom|tryHit
  (if (Variables|Default|GetisPlayerNear)
    (if (Variables|Default|GetneedsHits)
      (CallFunction|UpdateRequiredHits 1))))

(event Collision|EventActorEndOverlap
  (params (OtherActor :type Actor%20Object%20Reference))
  ;[1 1 1] Is player near?
  (if (Utilities|ClassIsChildOf (Utilities|GetClass OtherActor) "/Game/Blueprints/Blueprints/ThirdPersonCharacter.ThirdPersonCharacter_C")
    (Variables|Default|SetisPlayerNear false)
    (Variables|/Game/Blueprints/Blueprints/ThirdPersonCharacter.ThirdPersonCharacter_C|SetwrenchTarget (Variables|Default|GetnearPlayer) 0)
    (Variables|Default|SetnearPlayer 0)))

(event EventBeginPlay
  ;[1 1 1] Allows input
  (Input|EnableInput (Game|GetPlayerController 0))
  (CallFunction|UpdateRequiredHits))

(event EventTick
  (params (DeltaSeconds :type Float%20%28single-precision%29))
  (CallFunction|TextBillboard))

(event Collision|EventActorBeginOverlap
  (params (OtherActor :type Actor%20Object%20Reference))
  ;[1 1 1] Is player near?
  (if (Variables|Default|GetneedsHits)
    (if (Utilities|ClassIsChildOf (Utilities|GetClass OtherActor) "/Game/Blueprints/Blueprints/ThirdPersonCharacter.ThirdPersonCharacter_C")
      (Variables|Default|SetisPlayerNear true)
      (bind _asthird_person_character (Utilities|Casting|CastToThirdPersonCharacter OtherActor))
      (bind _output_get (Variables|Default|SetnearPlayer _asthird_person_character))
      (Variables|/Game/Blueprints/Blueprints/ThirdPersonCharacter.ThirdPersonCharacter_C|SetwrenchTarget _output_get self))))

(event Input|GamepadEvents|GamepadFaceButtonBottom
  (params (Key :type Key%20Structure)))

(fn ConstructionScript)

(fn TextBillboard
  (bind _returnvalue (Game|GetPlayerCameraManager 0))
  (Utilities|IsValid _returnvalue
    (:Is%20Valid
      (Transformation|SetWorldRotation (Variables|Default|GetnumHits) (Math|Rotator|FindLookatRotation (Transformation|GetWorldLocation (Variables|Default|GetnumHits)) (Camera|GetCameraLocation _returnvalue)) false false))))

(fn UpdateRequiredHits
  (params (numSubtract :type Integer))
  (if (> (Variables|Default|GetnumHitsReq) 0)
    (Variables|Default|SetnumHitsReq (- (Variables|Default|GetnumHitsReq) numSubtract))
    (bind _ashits_widget (Utilities|Casting|CastTohitsWidget (UserInterface|GetUserWidgetObject (Variables|Default|GetnumHits))))
    (Rendering|Components|TextRender|SetText (Variables|/Game/Blueprints/Blueprints/hitsWidget.hitsWidget_C|GetnumLeftText _ashits_widget) (Utilities|Text|ToText(String) (Utilities|String|Append (Utilities|String|Append (Utilities|String|ToString(Integer) (Variables|Default|GetnumHitsReq)) "/") (Utilities|String|ToString(Integer) (Variables|Default|GettotalHitsReq)))))
    (if (> numSubtract 0)
      (Audio|PlaySoundatLocation "/Game/Sound/wrench_hit_build_fail.wrench_hit_build_fail" "0, 0, 0" "0, 0, 0" 0.35))
    (else
      (Variables|Default|SetneedsHits false))))

(fn ReturnHits
  (return (Variables|Default|GetnumHitsReq)))