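; Carryable paint pickup that the third-person character can grab, drop and use as a source of a material.
; Grab and drop functions track the holder, and Tick snaps the actor to that character's HoldPosition while held.
; The cube's material is cached on BeginPlay and exposed through ReturnMat.
; DestroyPaint removes the paint only while held, first clearing the character's IsHolding flag.
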(event EventTick
  (params (DeltaSeconds :type Float%20%28single-precision%29))
  ;[1 1 1] Updating transform if held by the player
  (if true
    (if (Variables|Default|GetisHeld)
      (bind _asthird_person_character (Utilities|Casting|CastToThirdPersonCharacter (Variables|Default|GetOverlappedPlayer)))
      (Transformation|SetActorTransform (Transformation|GetWorldTransform (Variables|/Game/Blueprints/Blueprints/ThirdPersonCharacter.ThirdPersonCharacter_C|GetHoldPosition _asthird_person_character))))))

(event EventBeginPlay
  ;[1 1 1] Getting Material of the paint
  (Variables|Default|SetpaintMat (Rendering|Material|GetMaterial (Variables|Default|GetCube) 0))
  ;[1 1 1] Allows input on colorPaint
  (Input|EnableInput (Game|GetPlayerController 0)))

(fn ConstructionScript)

(fn DestroyPaint
  (if (Variables|Default|GetisHeld)
    (bind _asthird_person_character (Utilities|Casting|CastToThirdPersonCharacter (Variables|Default|GetOverlappedPlayer)))
    (Variables|/Game/Blueprints/Blueprints/ThirdPersonCharacter.ThirdPersonCharacter_C|SetisHolding _asthird_person_character false)
    (Actor|DestroyActor)))

(fn ReturnMat
  (return (Variables|Default|GetpaintMat)))

(fn PlayerGrab
  (params (playerInstagator :type Actor%20Object%20Reference))
  (if (not (Variables|Default|GetisHeld))
    (Variables|Default|SetOverlappedPlayer playerInstagator)
    (Variables|Default|SetisHeld true)))

(fn PlayerDrop
  (if (Variables|Default|GetisHeld)
    (Variables|Default|SetOverlappedPlayer 0)
    (Variables|Default|SetisHeld false)))