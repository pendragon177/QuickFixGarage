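; Fuel hose actor whose movable end (Ball7) can be grabbed, dropped or placed at a refueling position.
; While held, Tick snaps the end to the player's HoldPosition; otherwise the collider box follows it, with both paused during refueling.
; Dropping triggers a one-shot timeline that lerps the end back to ResetPoint.
; StartRefuel moves the end to the given position, disables its physics and clears the player's held-object state.
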(event EventTick
  (params (DeltaSeconds :type Float%20%28single-precision%29))
  (bind _ball7 (Variables|Components|Getball7))
  (if (not (Variables|Default|GetisRefuling))
    (Utilities|FlowControl|Sequence
      (:then_0
        (if (Variables|Default|GetisHeld)
          ;[1 1 1] Held By Player
          (bind _asthird_person_character (Utilities|Casting|CastToThirdPersonCharacter (Variables|Default|GetOverlappedPlayer)))
          (Transformation|SetWorldLocation _ball7 (.Location (Math|Transform|BreakTransform (Transformation|GetWorldTransform (Variables|/Game/Blueprints/Blueprints/ThirdPersonCharacter.ThirdPersonCharacter_C|GetHoldPosition _asthird_person_character)))) false false)
          (Transformation|SetWorldRotation _ball7 (.Rotation (Math|Transform|BreakTransform (Transformation|GetWorldTransform (Variables|/Game/Blueprints/Blueprints/ThirdPersonCharacter.ThirdPersonCharacter_C|GetHoldPosition _asthird_person_character)))) false false)
          (else
            ;[1 1 1] Updateing collider pos
            (Transformation|SetWorldLocation (Variables|Default|GetBox) (Transformation|GetWorldLocation (Variables|Components|Getball7)) false false))))
      (:then_1
        (if (Variables|Default|GetisResetting)
          (Utilities|FlowControl|DoOnce false :!label _label
            (:Completed
              (Variables|Default|SettempPos (Transformation|GetWorldLocation (Variables|Components|Getball7)))
              (bind _alpha (Timeline|restPos PlayFromStart)
                (:Update
                  (Transformation|SetWorldLocation (Variables|Components|Getball7) (Math|Vector|Lerp(Vector) (Variables|Default|GettempPos) (Transformation|GetWorldLocation (Variables|Default|GetresetPoint)) _alpha) false false))
                (:Finished
                  (Variables|Default|SetisResetting false)
                  (goto _label Reset))))))))))

(event EventBeginPlay
  ;[1 1 1] Allows input
  (Input|EnableInput (Game|GetPlayerController 0)))

(fn ConstructionScript)

(fn PlayerGrab
  (params (playerInstigator :type Actor%20Object%20Reference))
  (if (not (Variables|Default|GetisHeld))
    (Variables|Default|SetOverlappedPlayer playerInstigator)
    (Variables|Default|SetisHeld true)))

(fn PlayerDrop
  (if (Variables|Default|GetisHeld)
    (Variables|Default|SetOverlappedPlayer 0)
    (Variables|Default|SetisHeld false)
    (Variables|Default|SetisResetting true)
    (Variables|Default|SetisRefuling false)))

(fn StartRefuel
  (params (refulePos :type Vector))
  (Transformation|SetWorldLocation (Variables|Components|Getball7) refulePos false false)
  (Variables|Default|SetisRefuling true)
  (Physics|SetSimulatePhysics (Variables|Components|Getball7) false)
  (bind _asthird_person_character (Utilities|Casting|CastToThirdPersonCharacter (Variables|Default|GetOverlappedPlayer)))
  (Variables|/Game/Blueprints/Blueprints/ThirdPersonCharacter.ThirdPersonCharacter_C|SetisHolding _asthird_person_character false)
  (Variables|/Game/Blueprints/Blueprints/ThirdPersonCharacter.ThirdPersonCharacter_C|SetheldObject _asthird_person_character 0))