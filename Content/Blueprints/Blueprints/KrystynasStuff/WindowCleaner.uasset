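; WindowCleaner is a window cleaner item that a ThirdPersonCharacter can grab and carry.
; PlayerGrab stores the player, marks the item held and begins particle trails, while PlayerDrop clears that state and ends them.
; While held, Tick moves the root to the character's HoldPosition each frame instead of attaching it, adding 180 degrees of yaw so it faces forward.
; BeginPlay also enables input for the first player controller.
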(event EventBeginPlay
  (Input|EnableInput (Game|GetPlayerController 0)))

(event EventTick
  (params (DeltaSeconds :type Float%20%28single-precision%29))
  (if (Variables|Default|GetisHeld)
    (bind _asthird_person_character (Utilities|Casting|CastToThirdPersonCharacter (Variables|Default|GetOverlappedPlayer)))
    (Transformation|SetWorldLocationAndRotation (Variables|Default|GetDefaultSceneRoot) (.Location (Math|Transform|BreakTransform (Transformation|GetWorldTransform (Variables|/Game/Blueprints/Blueprints/ThirdPersonCharacter.ThirdPersonCharacter_C|GetHoldPosition _asthird_person_character)))) (Math|Rotator|MakeRotator (.Roll (Math|Rotator|BreakRotator (.Rotation (Math|Transform|BreakTransform (Transformation|GetWorldTransform (Variables|/Game/Blueprints/Blueprints/ThirdPersonCharacter.ThirdPersonCharacter_C|GetHoldPosition _asthird_person_character)))))) (.Pitch (Math|Rotator|BreakRotator (.Rotation (Math|Transform|BreakTransform (Transformation|GetWorldTransform (Variables|/Game/Blueprints/Blueprints/ThirdPersonCharacter.ThirdPersonCharacter_C|GetHoldPosition _asthird_person_character)))))) (+ (.Yaw (Math|Rotator|BreakRotator (.Rotation (Math|Transform|BreakTransform (Transformation|GetWorldTransform (Variables|/Game/Blueprints/Blueprints/ThirdPersonCharacter.ThirdPersonCharacter_C|GetHoldPosition _asthird_person_character)))))) 1.8e+02)) false false)))

(fn ConstructionScript)

(fn PlayerDrop
  (if (Variables|Default|GetisHeld)
    (Variables|Default|SetOverlappedPlayer 0)
    (Variables|Default|SetisHeld false)
    (Effects|Particles|Trails|EndTrails (Variables|Default|GetParticleSystem))))

(fn PlayerGrab
  (params (Player :type Actor%20Object%20Reference))
  (if (not (Variables|Default|GetisHeld))
    (Variables|Default|SetOverlappedPlayer Player)
    (Variables|Default|SetisHeld true)
    (Effects|Particles|Trails|BeginTrails (Variables|Default|GetParticleSystem) "None" "None" "ETrailWidthMode_FromCentre" 0.0)))