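; Car battery pickup actor that a ThirdPersonCharacter can carry and charge at a batteryChargeStation.
; Grab and drop functions track the holder, and Tick snaps the battery to that character's HoldPosition while held.
; Overlapping a station with BatteryAtStation set steps Timer down and swaps DeadBatterySprite in one pass without delays, setting BatteryCharged from SetSprite's result.
; BatteryDestroy clears the holder's IsHolding flag and destroys the actor.
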(event EventBeginPlay
  ;[1 1 1] Input on Battery Pickup
  (Input|EnableInput (Game|GetPlayerController 0)))

(event EventTick
  (params (DeltaSeconds :type Float%20%28single-precision%29))
  ;[1 1 1] Pickup Battery
  (if (Variables|Default|GetisHeld)
    (bind _asthird_person_character (Utilities|Casting|CastToThirdPersonCharacter (Variables|Default|GetOverlappedPlayer)))
    (Transformation|SetActorTransform (Transformation|GetWorldTransform (Variables|/Game/Blueprints/Blueprints/ThirdPersonCharacter.ThirdPersonCharacter_C|GetHoldPosition _asthird_person_character)))))

(event Collision|EventActorBeginOverlap
  (params (OtherActor :type Actor%20Object%20Reference))
  (Utilities|Casting|CastTobatteryChargeStation OtherActor)
  (if (Variables|Default|GetbatteryAtStation)
    (if (not (Variables|Default|GetbatteryCharged))
      (bind _output_get (Variables|Default|SetTimer (- (Variables|Default|GetTimer) 1.0)))
      (Rendering|Components|Sprite|SetSprite (Variables|Default|GetDeadBatterySprite) 0)
      (bind _output_get_2 (Variables|Default|SetTimer (- _output_get 1.0)))
      (Rendering|Components|Sprite|SetSprite (Variables|Default|GetDeadBatterySprite) 0)
      (bind _output_get_3 (Variables|Default|SetTimer (- _output_get_2 1.0)))
      (bind _returnvalue (Rendering|Components|Sprite|SetSprite (Variables|Default|GetDeadBatterySprite) 0))
      (Variables|Default|SetTimer (- _output_get_3 1.0))
      (Variables|Default|SetbatteryCharged _returnvalue))
    (else
      (Variables|Default|SetTimer (Variables|Default|GetTimer))
      (Rendering|Components|Sprite|SetSprite (Variables|Default|GetDeadBatterySprite) 0))))

(fn ConstructionScript)

(fn PlayerDrop
  (if (Variables|Default|GetisHeld)
    (Variables|Default|SetOverlappedPlayer 0)
    (Variables|Default|SetisHeld false)))

(fn PlayerGrab
  (params (Player :type Actor%20Object%20Reference))
  (if (not (Variables|Default|GetisHeld))
    (Variables|Default|SetOverlappedPlayer Player)
    (Variables|Default|SetisHeld true)))

(fn BatteryDestroy
  (if (Variables|Default|GetisHeld)
    (bind _asthird_person_character (Utilities|Casting|CastToThirdPersonCharacter (Variables|Default|GetOverlappedPlayer)))
    (Variables|/Game/Blueprints/Blueprints/ThirdPersonCharacter.ThirdPersonCharacter_C|SetisHolding _asthird_person_character false)
    (Actor|DestroyActor)))