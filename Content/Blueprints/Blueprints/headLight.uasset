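; Headlight pickup actor that a ThirdPersonCharacter can grab, carry and drop.
; Grab and drop functions toggle IsHeld and store or clear the holder, while Tick snaps the actor to that character's HoldPosition transform.
; DestroyHeadlight acts only while held, clearing the character's IsHolding flag, playing the Skrew sound at the world origin and destroying the actor.
; BeginPlay enables player 0 input, though no input events are defined here.
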(event EventBeginPlay
  ;[1 1 1] Allows input on pickupTire
  (Input|EnableInput (Game|GetPlayerController 0)))

(event EventTick
  (params (DeltaSeconds :type Float%20%28single-precision%29))
  ;[1 1 1] Updates transform if held by player
  (if (Variables|Default|GetisHeld)
    (bind _asthird_person_character (Utilities|Casting|CastToThirdPersonCharacter (Variables|Default|GetoverLappedPlayer)))
    (Transformation|SetActorTransform (Transformation|GetWorldTransform (Variables|/Game/Blueprints/Blueprints/ThirdPersonCharacter.ThirdPersonCharacter_C|GetHoldPosition _asthird_person_character)))))

(fn ConstructionScript)

(fn DestroyHeadlight
  (if (Variables|Default|GetisHeld)
    (bind _asthird_person_character (Utilities|Casting|CastToThirdPersonCharacter (Variables|Default|GetoverLappedPlayer)))
    (Variables|/Game/Blueprints/Blueprints/ThirdPersonCharacter.ThirdPersonCharacter_C|SetisHolding _asthird_person_character false)
    (Audio|PlaySoundatLocation "/Game/Sound/skrew.skrew" "0, 0, 0" "0, 0, 0" 0.65 0.55)
    (Actor|DestroyActor)))

(fn PlayerGrab
  (params (Player%20Instigator :type Actor%20Object%20Reference))
  (if (not (Variables|Default|GetisHeld))
    (Variables|Default|SetoverLappedPlayer Player%20Instigator)
    (Variables|Default|SetisHeld true)))

(fn PlayerDrop
  (if (Variables|Default|GetisHeld)
    (Variables|Default|SetoverLappedPlayer 0)
    (Variables|Default|SetisHeld false)))