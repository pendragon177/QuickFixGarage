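; MultiplayerTest runs a timed local multiplayer session built around a shared car.
; On BeginPlay it creates local players, spawns and possesses one ThirdPersonCharacter per GameInstanceMulti player count, and spawns a CarControl.
; Until time runs out, Tick drives a minutes-and-seconds countdown through a one-second Delay, respawning the car whenever invalid.
; Custom events handle car score and fix score; SpawnPaint is an empty stub.
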(event Custom|AddCarScore
  (params (CarScore :type Integer))
  (Variables|Default|SetScore (+ CarScore (Variables|Default|GetScore))))

(event Custom|AddCarFixScore
  (params (FixScore :type Integer))
  (Variables|Default|SetFixScore (+ (Variables|Default|GetFixScore) FixScore)))

(event EventBeginPlay
  (CallFunction|SpawnPlayers)
  (CallFunction|SpawnCar))

(event EventTick
  (params (DeltaSeconds :type Float%20%28single-precision%29))
  (if (not (Variables|Default|GetisTimerDone))
    (Utilities|FlowControl|Sequence
      (:then_0
        (bind _isdone (CallFunction|CheckTimer))
        (Variables|Default|SetisTimerDone _isdone))
      (:then_1
        (if (Utilities|IsValid (Variables|Default|GetLevelCar))
          ;[1 1 1] Countdown Timer
          (Utilities|FlowControl|Delay 1.0)
          (Variables|Default|SetSeconds (- (Variables|Default|GetSeconds) 1))
          (if (< (Variables|Default|GetSeconds) 0)
            (Variables|Default|SetMinutes (- (Variables|Default|GetMinutes) 1))
            (Variables|Default|SetSeconds 59))
          (else
            (CallFunction|SpawnCar)))))))

(fn ConstructionScript)

(fn SpawnPlayers
  (bind _asgame_instance_multi (Utilities|Casting|CastToGameInstanceMulti (Game|GetGameInstance)))
  (for _index (range 1 2)
    (Class|GameplayStatics|CreatePlayer _index))
  (for _index_2 (range 0 (- (Variables|/Game/Blueprints/Maps/GameInstanceMulti.GameInstanceMulti_C|GetPlayerCount _asgame_instance_multi) 1))
    (bind _returnvalue (Game|SpawnActorfromClass "/Game/Blueprints/Blueprints/ThirdPersonCharacter.ThirdPersonCharacter_C" (Math|Transform|MakeTransform "0, 0,2000.000000") "Undefined" 0 _index_2 0))
    (Pawn|Possess (Game|GetPlayerController _index_2) _returnvalue)))

(fn SpawnCar
  (bind _returnvalue (Game|SpawnActorfromClass "/Game/Blueprints/Blueprints/CarControl.CarControl_C" (Math|Transform|MakeTransform "0, 0, 0") "Undefined" 0 0))
  (Variables|Default|SetLevelCar _returnvalue))

(fn SpawnPaint)

(fn CheckTimer
  (return (and (<= (Variables|Default|GetMinutes) 0) (<= (Variables|Default|GetSeconds) 0))))